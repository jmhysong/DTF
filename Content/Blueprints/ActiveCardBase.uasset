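; Base actor for a clickable card that highlights under the cursor and spawns a visual card near the player when clicked.
; On click, it spawns a VisualCardBase at the player capsule, offsets it along world X toward the origin side, and sets its mesh rotation by the sign of the player's X.
; Cursor-over events, bound on BeginPlay, toggle custom depth rendering with a stencil value for the highlight.
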(event `self.ReceiveActorOnClicked`
  (bind _returnvalue (`SceneComponent.K2_GetComponentToWorld` (`Character.CapsuleComponent` (`GameplayStatics.GetPlayerCharacter` 0))))
  (bind _returnvalue_2 (`KismetMathLibrary.MakeVector` (.x (.location _returnvalue)) (.y (.location _returnvalue)) (.z (.location _returnvalue))))
  (bind _returnvalue_3 (`|SpawnActorFromClass` "/Game/Blueprints/VisualCardBase.VisualCardBase_C" _returnvalue "AlwaysSpawn" "OverrideRootScale"))
  (if (> (.x (.location _returnvalue)) 0.0)
    (`self.K2_SetActorRelativeLocation` _returnvalue_3 (- _returnvalue_2 (250.0 0.0 0.0)) false false)
    (`SceneComponent.K2_SetRelativeRotation` (`StaticMeshActor.StaticMeshComponent` _returnvalue_3) (.rotation _returnvalue) false false)
    (else
      (`self.K2_SetActorRelativeLocation` _returnvalue_3 (+ _returnvalue_2 (250.0 0.0 0.0)) false false)
      (`SceneComponent.K2_SetRelativeRotation` :`self` (`StaticMeshActor.StaticMeshComponent` _returnvalue_3)))))

(event `self.ReceiveActorBeginOverlap`
  (params (OtherActor :type "Actor Object Reference")))

(event `self.ReceiveBeginPlay`
  (`|ExecutionSequence`
    (:`then_0`
      (add `self.OnBeginCursorOver` (delegate `OnBeginCursorOver_Event_0`)))
    (:`then_1`
      (add `self.OnEndCursorOver` (delegate `OnEndCursorOver_Event_0`)))))

(event `self.ReceiveTick`
  (params (DeltaSeconds :type "Float (single-precision)")))

(event `OnBeginCursorOver_Event_0`
  (`PrimitiveComponent.SetRenderCustomDepth` (`self.StaticMeshComponent`) true)
  (`PrimitiveComponent.SetCustomDepthStencilValue` (`self.StaticMeshComponent`) 252))

(event `OnEndCursorOver_Event_0`
  (`PrimitiveComponent.SetRenderCustomDepth` (`self.StaticMeshComponent`) false)
  (`PrimitiveComponent.SetCustomDepthStencilValue` (`self.StaticMeshComponent`) 252))

(fn `UserConstructionScript`)