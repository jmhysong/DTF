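; Chat system component that gives the local player a multiplayer chat HUD with tabbed groups, private messages and chat commands.
; Non-dedicated local owners spawn the widget, then create or join the Global and PMs groups by authority.
; Server-named events parse messages through GetChatCommand and track players and groups, some in the game instance.
; PushItem displays messages after mute checks, while other events manage tab switching, removal and keyboard focus.
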(event `self.ReceiveBeginPlay`
  (bind _returnvalue (`self.GetOwner`))
  ;[1 1 1] Initialize the chat
  (`KismetSystemLibrary.Delay` 0.2)
  (bind _asdtfgame_instance_bp (cast `/Game/Blueprints/DTFGameInstanceBP` (`GameplayStatics.GetGameInstance`)))
  (set `self.Game Instance Blueprint` _asdtfgame_instance_bp)
  (if (and (or (== _returnvalue (`GameplayStatics.GetPlayerCharacter` 0)) (== _returnvalue (`GameplayStatics.GetPlayerController` 0)) (== _returnvalue (`GameplayStatics.GetPlayerPawn` 0))) (not (`KismetSystemLibrary.IsDedicatedServer`)))
    (`self.Spawn Chat`)))

(event `Spawn Chat`
  ;[1 1 1] Add HUD widget
  (bind _returnvalue (`|CreateWidget` "/Game/Blueprints/DTFHUDBP.DTFHUDBP_C" (`GameplayStatics.GetPlayerController` 0) self))
  (bind _output_get (set `self.Chat Widget` (`/Game/Blueprints/DTFHUDBP.Chat Widget` _returnvalue)))
  (set `/Game/BPChatSystem/Blueprints/Chat_MainWidget.Chat System` self _output_get)
  (`UserWidget.AddToViewport` _returnvalue 0)
  (`self.Add Player to Chat`)
  (`/Engine/EditorBlueprintResources/ActorMacros.Switch Has Authority`
    (:`Authority`
      (`self.Create Group` "Global")
      (`self.Create Group` "PMs"))
    (:`Remote`
      (`self.Join Group` "Global")
      (`self.Join Group` "PMs"))))

(event `Send Chat Message Server`
  (params (Message :type String) (Group :type String))
  (bind _players_to_message (`self.Players to Message`))
  ;[1 1 1] Send Chat Message on Server
  (bind (_command_result _new_message _new_group) (`/Game/BPChatSystem/Blueprints/Chat_FL.Get Chat Command` Message self Group))
  (switch `/Game/BPChatSystem/Blueprints/Enums/Command_Returns` _command_result
    (:`NewEnumerator0`
      (for _array_element (`self.Players to Message`)
        (`self.Push Item` _array_element null self _new_message _new_group true) ; Push the item, but don't use the 'To:' input, as using it will append 'To:' to the username, which is for private messaging
      ))
    (:`NewEnumerator1`
      (for _array_element_2 _players_to_message
        (`self.Push Item` _array_element_2 (`KismetArrayLibrary.Array_Get` _players_to_message) self _new_message _new_group true) ; Push the item, use the 'To:' input so that 'To' or 'From' will be appended to the username due to it being a private message
      ))
    (:`NewEnumerator5`
      (`self.Push Item` null self _new_message _new_group false :!label _label) ; Push the message, but don't display a username since the message is a return message, such as 'You have joined the group _______'
    )
    (:`NewEnumerator6`
      (goto _label))
    (:`NewEnumerator7`
      (goto _label))
    (:`NewEnumerator9`
      (goto _label))
    (:`NewEnumerator10`
      (goto _label))
    (:`NewEnumerator11`
      (goto _label))
    (:`NewEnumerator12`
      (goto _label))
    (:`NewEnumerator13`
      (goto _label))
    (:`NewEnumerator4`
      (goto _label))
    (:`NewEnumerator3`
      (goto _label))))

(event `Add Local Group on Server`
  (params (`Group Name` :type String))
  ;[1 1 1] Custom Events for leaving/joining groups
  (`KismetArrayLibrary.Array_Add` (`self.Joined Groups`) `Group Name`))

(event `Remove Local Group on Server`
  (params (`Group Name` :type String))
  ;[1 1 1] Custom Events for leaving/joining groups
  (`KismetArrayLibrary.Array_RemoveItem` (`self.Joined Groups`) `Group Name`))

(event `Create Group`
  (params (`Group Name` :type String))
  ;[1 1 1] Create Group
  (`self.Add Global Group on Server` `Group Name`)
  (`self.Add Owned Group on Server` `Group Name`) ; Give ourselves ownership of the group, since we created it
  (`self.Join Group` `Group Name`))

(event `Add Owned Group on Server`
  (params (Group :type String))
  ;[1 1 1] Custom Events for leaving/joining groups
  (`KismetArrayLibrary.Array_Add` (`self.Owned Groups`) Group))

(event `Remove Owned Group On Server`
  (params (Group :type String))
  ;[1 1 1] Custom Events for leaving/joining groups
  (`KismetArrayLibrary.Array_RemoveItem` (`self.Owned Groups`) Group))

(event `Add Global Group on Server`
  (params (Group :type String))
  ;[1 1 1] Custom Events for leaving/joining groups
  (`KismetArrayLibrary.Array_Add` (`/Game/Blueprints/DTFGameInstanceBP.Chat Groups` (`self.Game Instance Blueprint`)) Group))

(event `Join Group`
  (params (`Group Name` :type String))
  ;[1 1 1] Join Group
  (bind _returnvalue (`|CreateWidget` "/Game/BPChatSystem/Blueprints/ComponentWidgets/Chat_DialogBox.Chat_DialogBox_C" (`GameplayStatics.GetPlayerController` 0) `Group Name`))
  (`PanelWidget.AddChild` (`/Game/BPChatSystem/Blueprints/Chat_MainWidget.Chat Switcher` (`self.Chat Widget`)) _returnvalue)
  (bind _returnvalue_2 (`|CreateWidget` "/Game/BPChatSystem/Blueprints/ComponentWidgets/Chat_Tab.Chat_Tab_C" (`GameplayStatics.GetPlayerController` 0) (`KismetTextLibrary.Conv_StringToText` `Group Name`) (`self.Chat Widget`) _returnvalue))
  (`PanelWidget.AddChild` (`/Game/BPChatSystem/Blueprints/Chat_MainWidget.Tab Scrollbox` (`self.Chat Widget`)) _returnvalue_2)
  (`self.Add Local Group on Server` `Group Name`))

(event `Leave Group`
  (params (`Group Name` :type String) (Index :type Integer))
  (bind _chat_widget (`self.Chat Widget`))
  (bind _chat_switcher (`/Game/BPChatSystem/Blueprints/Chat_MainWidget.Chat Switcher` (`self.Chat Widget`)))
  (bind _returnvalue (`WidgetSwitcher.GetActiveWidgetIndex` _chat_switcher))
  (bind _returnvalue_2 (== _returnvalue (- (`PanelWidget.GetChildrenCount` _chat_switcher) 1)))
  ;[1 1 1] Leave Group
  (if (== Index _returnvalue)
    (`/Game/BPChatSystem/Blueprints/ComponentWidgets/Chat_Tab.Set as Active Tab` (cast `/Game/BPChatSystem/Blueprints/ComponentWidgets/Chat_Tab` (`PanelWidget.GetChildAt` (`/Game/BPChatSystem/Blueprints/Chat_MainWidget.Tab Scrollbox` (`self.Chat Widget`)) (+ _returnvalue (`KismetMathLibrary.SelectInt` -1 1 _returnvalue_2))) :!pure true))
    (`WidgetSwitcher.SetActiveWidgetIndex` _chat_switcher (+ _returnvalue (`KismetMathLibrary.SelectInt` -1 0 _returnvalue_2)) :!label _label_2)
    (elif (> _returnvalue Index)
      (goto _label_2)
      (else
        _)))
  (`PanelWidget.RemoveChildAt` (`/Game/BPChatSystem/Blueprints/Chat_MainWidget.Chat Switcher` _chat_widget) Index)
  (`PanelWidget.RemoveChildAt` (`/Game/BPChatSystem/Blueprints/Chat_MainWidget.Tab Scrollbox` _chat_widget) Index)
  (`self.Remove Local Group on Server` `Group Name`)
  (if (`KismetArrayLibrary.Array_Contains` (`self.Owned Groups`) `Group Name`)
    (`self.Remove Owned Group On Server` `Group Name`)))

(event `Push Item`
  (params (`To:` :type "/Game/BPChatSystem/Blueprints/Chat_System Object Reference") (`From:` :type "/Game/BPChatSystem/Blueprints/Chat_System Object Reference") (Message :type String) (Group :type String) (`Display Username?` :type Boolean))
  (bind _player_name (`/Game/BPChatSystem/Blueprints/Chat_System.Player Name` `From:`))
  (bind _returnvalue (== `From:` self))
  ;[1 1 1] Push Item
  (if (`KismetArrayLibrary.Array_Contains` (`self.Muted Players`) `From:`)
    _
    (elif (not (and (`KismetArrayLibrary.Array_Contains` (`/Game/BPChatSystem/Blueprints/Chat_System.Muted Players` `From:`) self) (`self.Two-way Mute?`)))
      (`/Engine/EditorBlueprintResources/StandardMacros.IsValid` `To:`
        (:`Is Valid`
          (`/Game/BPChatSystem/Blueprints/Chat_MainWidget.PushItem` (`self.Chat Widget`) (`KismetMathLibrary.SelectString` (`KismetStringLibrary.Concat_StrStr` (`KismetMathLibrary.SelectString` "To " "From " _returnvalue) (`KismetMathLibrary.SelectString` (`/Game/BPChatSystem/Blueprints/Chat_System.Player Name` `To:`) _player_name _returnvalue)) "" `Display Username?`) Message Group) ; Since the 'To:' input is valid, we are sending a private message, so append 'To:' or 'From:' to the username
        )
        (:`Is Not Valid`
          (`/Game/BPChatSystem/Blueprints/Chat_MainWidget.PushItem` (`self.Chat Widget`) (`KismetMathLibrary.SelectString` _player_name "" `Display Username?`) Message Group) ; Since the 'To:' input IS NOT valid, we are not sending a private message, so just use the player's normal username
        )))))

(event `Set Keyboard Focus to Chat Input`
  (bind _chat_widget (`self.Chat Widget`))
  ;[1 1 1] Set Chat Keyboard Focus
  (`/Engine/EditorBlueprintResources/StandardMacros.IsValid` _chat_widget
    (:`Is Valid`
      (`/Game/BPChatSystem/Blueprints/Chat_MainWidget.Set Keyboard Focus` _chat_widget))))

(event `Add Player to Chat`
  ;[1 1 1] Add player to chat
  (`KismetArrayLibrary.Array_Add` (`/Game/Blueprints/DTFGameInstanceBP.Players in Chat` (`self.Game Instance Blueprint`)) self))

(event `Previous/Next Tab`
  (params (Direction :type "/Game/BPChatSystem/Blueprints/Enums/Tab_Direction Enum") (`Wrap Around at End?` :type Boolean))
  (bind _chat_widget (`self.Chat Widget`))
  (bind _chat_widget_2 (`self.Chat Widget`))
  (bind _chat_switcher (`/Game/BPChatSystem/Blueprints/Chat_MainWidget.Chat Switcher` (`self.Chat Widget`)))
  (bind _tab_scrollbox (`/Game/BPChatSystem/Blueprints/Chat_MainWidget.Tab Scrollbox` (`self.Chat Widget`)))
  (bind _returnvalue (`WidgetSwitcher.GetActiveWidgetIndex` _chat_switcher))
  ;[1 1 1] Previous/Next Tab
  (switch `/Game/BPChatSystem/Blueprints/Enums/Tab_Direction` Direction
    (:`NewEnumerator0`
      (if (== _returnvalue 0)
        (if `Wrap Around at End?`
          (bind _aschat_tab (cast `/Game/BPChatSystem/Blueprints/ComponentWidgets/Chat_Tab` (`PanelWidget.GetChildAt` _tab_scrollbox (- (`PanelWidget.GetChildrenCount` _tab_scrollbox) 1))))
          (`/Game/BPChatSystem/Blueprints/ComponentWidgets/Chat_Tab.Set as Active Tab` _aschat_tab) ; Set the right-most tab to be active since we wrapped around from the very left
        )
        (else
          (bind _aschat_tab_2 (cast `/Game/BPChatSystem/Blueprints/ComponentWidgets/Chat_Tab` (`PanelWidget.GetChildAt` (`/Game/BPChatSystem/Blueprints/Chat_MainWidget.Tab Scrollbox` _chat_widget) (- (`WidgetSwitcher.GetActiveWidgetIndex` (`/Game/BPChatSystem/Blueprints/Chat_MainWidget.Chat Switcher` _chat_widget)) 1))))
          (`/Game/BPChatSystem/Blueprints/ComponentWidgets/Chat_Tab.Set as Active Tab` _aschat_tab_2) ; Set the tab to the left of the current active tab to be active
        )))
    (:`NewEnumerator1`
      (if (== (+ _returnvalue 1) (`PanelWidget.GetChildrenCount` _chat_switcher))
        (if `Wrap Around at End?`
          (bind _aschat_tab_3 (cast `/Game/BPChatSystem/Blueprints/ComponentWidgets/Chat_Tab` (`PanelWidget.GetChildAt` (`/Game/BPChatSystem/Blueprints/Chat_MainWidget.Tab Scrollbox` (`self.Chat Widget`)) 0)))
          (`/Game/BPChatSystem/Blueprints/ComponentWidgets/Chat_Tab.Set as Active Tab` _aschat_tab_3) ; Set theleftt-most tab to be active since we wrapped around from the very right
        )
        (else
          (bind _aschat_tab_4 (cast `/Game/BPChatSystem/Blueprints/ComponentWidgets/Chat_Tab` (`PanelWidget.GetChildAt` (`/Game/BPChatSystem/Blueprints/Chat_MainWidget.Tab Scrollbox` _chat_widget_2) (+ (`WidgetSwitcher.GetActiveWidgetIndex` (`/Game/BPChatSystem/Blueprints/Chat_MainWidget.Chat Switcher` _chat_widget_2)) 1))))
          (`/Game/BPChatSystem/Blueprints/ComponentWidgets/Chat_Tab.Set as Active Tab` _aschat_tab_4) ; Set the tab to the right of the current active tab to be active
        )))))

(fn `Get Current Group`
  (returns (Group :type String))
  (return (`/Game/BPChatSystem/Blueprints/ComponentWidgets/Chat_DialogBox.Group` (`/Game/BPChatSystem/Blueprints/Chat_MainWidget.CurrentDialogBox` (`self.Chat Widget`)))))

(fn `Send Chat Message`
  (params (Message :type String) (Group :type String))
  (if (`/Game/BPChatSystem/Blueprints/Chat_FL.Get String Validity` Message)
    (`self.Send Chat Message Server` Message Group))
  (return))

(fn `UserConstructionScript`)